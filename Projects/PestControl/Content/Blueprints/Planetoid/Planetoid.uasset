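; Planetoid actor that forms a body from overlapping icosahedron instances and serves as its own orbit-camera view.
; On BeginPlay it becomes the player's view target and adds instanced icosahedrons at one shared origin, each randomly rotated and uniformly scaled.
; Each tick, mouse movement rotates the camera arm with clamped pitch.
; An input axis slides the camera along local X for zoom, within limits proportional to the planetoid's scale.
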(event EventTick
  (params (DeltaSeconds :type Float%20%28single-precision%29))
  (bind _returnvalue (Game|GetPlayerController 0))
  (bind _scale (Variables|Default|GetScale))
  (bind _cameraspeed (Variables|Default|GetCameraSpeed))
  (bind _camera (Variables|Default|GetCamera))
  (bind _arm (Variables|Default|GetArm))
  (bind (_deltax _deltay) (Class|PlayerController|GetInputMouseDelta _returnvalue))
  (bind _relativelocation (Variables|/Script/Engine.SceneComponent|GetRelativeLocation _camera))
  (bind _relativerotation (Variables|/Script/Engine.SceneComponent|GetRelativeRotation _arm))
  (bind (_roll _pitch _yaw) (Math|Rotator|BreakRotator _relativerotation))
  (bind (_x _y _z) (Math|Vector|BreakVector _relativelocation))
  ;[1 1 1] Camera Rotation
  (Transformation|SetRelativeRotation (Variables|Default|GetArm) (Math|Rotator|MakeRotator _roll (Math|Float|Clamp(Float) (+ _pitch (* _deltay _cameraspeed)) (Variables|Default|GetMinimumPitch) (Variables|Default|GetMaximumPitch)) (+ _yaw (* _deltax _cameraspeed))) false false)
  ;[1 1 1] Camera Zoom
  (Transformation|SetRelativeLocation (Variables|Default|GetCamera) (Math|Vector|MakeVector (Math|Float|Clamp(Float) (+ _x (* (Class|Actor|GetInputAxisKeyValue) (Variables|Default|GetZoomSpeed))) (* (Variables|Default|GetMaximumZoom) _scale -1.0) (* (Variables|Default|GetMinimumZoom) _scale -1.0)) _y _z) false false))

(event EventBeginPlay
  ;[1 1 1] Set Camera
  (Game|Player|SetViewTargetwithBlend (Game|GetPlayerController 0) self 0.0 "VTBlend_Linear" 0.0 false)
  ;[1 1 1] Spawn Icosahedrons
  (for _index (range 1 (Variables|Default|GetNumberOfIcosahedrons))
    (Components|InstancedStaticMesh|AddInstance (Variables|Default|GetIcosahedron) (Math|Transform|MakeTransform "0, 0, 0" (Math|Random|RandomRotator true) (Math|Conversions|ToVector(Float) (/ (Variables|Default|GetScale) (Variables|Default|GetImportScale)))))))

(fn ConstructionScript)