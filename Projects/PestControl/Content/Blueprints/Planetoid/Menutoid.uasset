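; Menutoid is a decorative planetoid actor that, judging by its name, serves as a menu backdrop and becomes player 0's view target on BeginPlay.
; It builds the planetoid by stacking a configurable number of randomly rotated, uniformly scaled icosahedron instances at the local origin of one instanced mesh component.
; Tick yaws that component at RotationSpeed, spinning the whole cluster as one.
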(event EventBeginPlay
  ;[1 1 1] Set Camera
  (Game|Player|SetViewTargetwithBlend (Game|GetPlayerController 0) self 0.0 "VTBlend_Linear" 0.0 false)
  ;[1 1 1] Spawn Icosahedrons
  (for _index (range 1 (Variables|Default|GetNumberOfIcosahedrons))
    (Components|InstancedStaticMesh|AddInstance (Variables|Default|GetIcosahedron) (Math|Transform|MakeTransform "0, 0, 0" (Math|Random|RandomRotator true) (Math|Conversions|ToVector(Float) (/ (Variables|Default|GetScale) (Variables|Default|GetImportScale)))))))

(event EventTick
  (params (DeltaSeconds :type Float%20%28single-precision%29))
  ;[1 1 1] Rotate Planetoid
  (Transformation|AddLocalRotation (Variables|Default|GetIcosahedron) (Math|Rotator|MakeRotator 0.0 0.0 (* DeltaSeconds (Variables|Default|GetRotationSpeed))) false false))

(fn ConstructionScript)