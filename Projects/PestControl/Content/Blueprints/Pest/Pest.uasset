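; Pest creature that hops toward a navigation target, currently hardcoded, as a physics sphere pulled by gravity toward the world origin.
; Randomly timed impulses drive it, scaled by closeness and slope.
; A trace toward the origin supplies the surface normal, switching physical material and damping between uphill and downhill.
; A periodically recorded position feeds a randomized check for lingering in place, which so far only prints a placeholder message.
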(event EventBeginPlay
  (Utilities|FlowControl|Sequence
    (:then_0
      ;[1 1 1] Occasionally Bump
      (Utilities|FlowControl|Delay (Math|Random|RandomFloatinRange (Variables|Default|GetMinimumDelay) (Variables|Default|GetMaximumDelay)) :!label _label)
      (Variables|Default|SetShouldBump true)
      (goto _label))
    (:then_1
      ;[1 1 1] Record Position
      (Utilities|FlowControl|Delay (Variables|Default|GetGraceDuration) :!label _label_2)
      (Variables|Default|SetGracePosition (Transformation|GetActorLocation))
      (Variables|Default|SetGraceTime (Utilities|Time|GetTimeSeconds))
      (goto _label_2))))

(event EventTick
  (params (DeltaSeconds :type Float%20%28single-precision%29))
  (bind _sphere (Variables|Default|GetSphere))
  ;[1 1 1] Apply Gravity
  (Physics|AddForce (Variables|Default|GetSphere) (* (Math|Vector|NegateVector (Math|Vector|Normalize (Transformation|GetActorLocation))) (Variables|Default|GetGravity)) "None" false)
  (Utilities|FlowControl|Sequence
    (:then_0
      (Utilities|FlowControl|Sequence
        (:then_0
          (Variables|Default|SetNavigationTarget "10000.000000, 0, 0"))
        (:then_1
          ;[1 1 1] Calculate Navigation Normal
          (bind (_outhit _returnvalue) (Collision|LineTraceForObjects (Transformation|GetActorLocation) "0.000000, 0, 0" (Utilities|Array|MakeArray "ObjectTypeQuery1" "ObjectTypeQuery2") false 0 "None"))
          (if _returnvalue
            (Variables|Default|SetNavigationNormal (.ImpactNormal (Collision|BreakHitResult _outhit)))))))
    (:then_1
      (Utilities|FlowControl|Sequence
        (:then_0
          ;[1 1 1] Stop While Close
          (Variables|Default|SetBumpIntensityWhileClose (Class|PestBase|GetNavigationRange (Variables|Default|GetMinimumCloseRange) (Variables|Default|GetMaximumCloseRange))))
        (:then_1
          ;[1 1 1] Horny Check
          (if (< (Math|Random|RandomFloatinRange 0.0 (Variables|Default|GetGraceDuration)) (- (Utilities|Time|GetTimeSeconds) (Variables|Default|GetGraceTime)))
            (if (< (Math|Vector|VectorLength (- (Transformation|GetActorLocation) (Variables|Default|GetGracePosition))) (Variables|Default|GetGraceRange))
              (Development|PrintString "It's fucking time!"))))))
    (:then_2
      ;[1 1 1] Uphill/Downhill
      (if (< (Math|Vector|DotProduct (Variables|Default|GetNavigationNormal) (Class|PestBase|GetNavigationDirection)) 0.0)
        (Class|PrimitiveComponent|SetPhysMaterialOverride _sphere "/Game/Blueprints/Pest/PestPhysicalMaterialUphill.PestPhysicalMaterialUphill")
        (Class|PrimitiveComponent|SetLinearDamping _sphere 1e+01)
        (Variables|Default|SetBumpIntensityWhileSliding 1.0)
        (else
          (Class|PrimitiveComponent|SetPhysMaterialOverride _sphere "/Game/Blueprints/Pest/PestPhysicalMaterialDownHill.PestPhysicalMaterialDownhill")
          (Class|PrimitiveComponent|SetLinearDamping _sphere 2.0)
          (Variables|Default|SetBumpIntensityWhileSliding (- 1.0 (Math|Vector|DotProduct (Variables|Default|GetNavigationNormal) (Class|PestBase|GetNavigationDirection)))))))
    (:then_3
      ;[1 1 1] Bump to Navigation Target
      (if (Variables|Default|GetShouldBump)
        (Physics|AddImpulse (Variables|Default|GetSphere) (* (Class|PestBase|GetNavigationDirection) (* (Variables|Default|GetBumpImpulse) (Variables|Default|GetBumpIntensityWhileSliding) (Variables|Default|GetBumpIntensityWhileClose))) "None" false)
        (Variables|Default|SetShouldBump false)))))

(fn ConstructionScript)