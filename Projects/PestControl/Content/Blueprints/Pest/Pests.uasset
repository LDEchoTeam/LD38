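; Manager actor that populates the planetoid with pests and handles their breeding.
; On BeginPlay it waits a frame for planetoid setup, then spawns a set number of pests at random directions above the surface.
; SpawnPest traces toward the world origin, placing each pest on the hit point aligned to the surface normal.
; Each tick, pairs of horny pests within a set distance spawn offspring at their midpoint and become satisfied.
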(event EventBeginPlay
  ;[1 1 1] Spawn Pests
  (Utilities|FlowControl|Delay 0.0) ; A delay of 0 waits one frame.
  (for _index (range 1 (Variables|Default|GetNumberOfPests))
    (CallFunction|SpawnPest (* (Math|Random|RandomUnitVector) (* (Variables|/Game/Blueprints/Planetoid/Planetoid.Planetoid_C|GetScale (Variables|/Game/Blueprints/Directory/Directory.Directory_C|GetPlanetoid (Variables|Default|GetDirectory))) 2.0))) ; Executed AFTER the planetoid is set up.
  ))

(event EventTick
  (params (DeltaSeconds :type Float%20%28single-precision%29))
  (bind _pests (Variables|Default|GetPests))
  (bind _returnvalue (Utilities|Array|Length _pests))
  (bind _returnvalue_2 (- _returnvalue 1))
  ;[1 1 1] Fornication
  (for _index (range 0 _returnvalue_2)
    (if (Variables|/Game/Blueprints/Pest/Pest.Pest_C|GetHorny (Utilities|Array|Get(acopy) (Variables|Default|GetPests) _index))
      (for _index_2 (range (+ _index 1) _returnvalue_2)
        (if (Variables|/Game/Blueprints/Pest/Pest.Pest_C|GetHorny (Utilities|Array|Get(acopy) (Variables|Default|GetPests) _index_2))
          (if (< (Transformation|GetDistanceTo (Utilities|Array|Get(acopy) (Variables|Default|GetPests) _index) (Utilities|Array|Get(acopy) (Variables|Default|GetPests) _index_2)) (Variables|Default|GetFuckCircle))
            (CallFunction|SpawnPest (/ (+ (Transformation|GetActorLocation (Utilities|Array|Get(acopy) (Variables|Default|GetPests) _index_2)) (Transformation|GetActorLocation (Utilities|Array|Get(acopy) (Variables|Default|GetPests) _index))) 2.0))
            (Default|Satisfaction (Utilities|Array|Get(acopy) (Variables|Default|GetPests) _index))
            (Default|Satisfaction (Utilities|Array|Get(acopy) (Variables|Default|GetPests) _index_2))))))))

(fn ConstructionScript)

(fn SpawnPest
  (params (Position :type Vector))
  (bind (_outhit _returnvalue) (Collision|LineTraceForObjects (* Position 2.0) "0.000000, 0, 0" (Utilities|Array|MakeArray "ObjectTypeQuery7") false 0 "None"))
  (if _returnvalue
    (bind _returnvalue_2 (Game|SpawnActorfromClass "/Game/Blueprints/Pest/Pest.Pest_C" (Math|Transform|MakeTransform (.ImpactPoint (Collision|BreakHitResult _outhit)) (Math|Rotator|MakeRotfromZX (.ImpactNormal (Collision|BreakHitResult _outhit)) (Math|Random|RandomUnitVector))) "AdjustIfPossibleButAlwaysSpawn" 0 0))
    (Utilities|Array|Add (Variables|Default|GetPests) _returnvalue_2)))