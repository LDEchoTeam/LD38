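; Visitors Blueprint that tracks park-style visitor attendance and converts it into score over time.
; A looping delay started at BeginPlay adjusts attendance by a happiness curve sampled on the Directory's pest count, minus the Lokator count.
; While attendance stays positive, it adds attendance-scaled points to the score and repeats.
; When attendance hits zero or below, it pauses the game as a placeholder fail state.
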(event EventBeginPlay
  ;[1 1 1] Attendence
  (Utilities|FlowControl|Delay (Variables|Default|GetAttendenceDelay) :!label _label)
  (bind _output_get (Variables|Default|SetAttendence (+ (Variables|Default|GetAttendence) (Math|Curves|GetFloatValue (Variables|Default|GetHappinessCurve) (Math|Conversions|ToFloat(Integer) (Utilities|Array|Length (Variables|/Game/Blueprints/Pest/Pests.Pests_C|GetPests (Variables|/Game/Blueprints/Directory/Directory.Directory_C|GetPests (Variables|Default|GetDirectory)))))) (* (Math|Conversions|ToFloat(Integer) (Utilities|Array|Length (Variables|/Game/Blueprints/Lokator/Lokators.Lokators_C|GetLokators (Variables|/Game/Blueprints/Directory/Directory.Directory_C|GetLokators (Variables|Default|GetDirectory))))) -1.0))))
  (if (> _output_get 0.0)
    ;[1 1 1] Score
    (Variables|Default|SetScore (+ (Variables|Default|GetScore) (* (Variables|Default|GetAttendenceScore) (Variables|Default|GetAttendence))))
    (goto _label)
    (else
      (Game|SetGamePaused true) ; TODO...
    )))

(event EventTick
  (params (DeltaSeconds :type Float%20%28single-precision%29))
  ;[1 1 1] Attendence
)

(fn ConstructionScript)