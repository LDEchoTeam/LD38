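; Manager Blueprint that spawns and selects Lokator actors on a spherical surface centered at the world origin.
; Space spawns a Lokator at the cursor hit, with its Z axis along the normalized hit position and a random X, then links it back and stores it.
; Left click selects the Lokator nearest the hit by dot product of normalized positions, showing only that one's Cone.
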(event EventBeginPlay)

(event EventTick
  (params (DeltaSeconds :type Float%20%28single-precision%29)))

(event Input|MouseEvents|LeftMouseButton
  (params (Key :type Key%20Structure :default "AnyKey"))
  (bind _returnvalue (Game|GetPlayerController 0))
  (bind _array (Utilities|Array|MakeArray "ObjectTypeQuery7"))
  (bind (_hitresult _returnvalue_2) (Class|PlayerController|GetHitResultUnderCursorforObjects _returnvalue _array false))
  (:Pressed
    (if _returnvalue_2
      (bind _lokator (CallFunction|FindClosestLokator (.ImpactPoint (Collision|BreakHitResult _hitresult))))
      (Utilities|IsValid _lokator
        (:Is%20Valid
          (Utilities|IsValid (Variables|Default|GetSelectedLokator)
            (:Is%20Valid
              (Rendering|SetVisibility (Variables|/Game/Blueprints/Lokator/Lokator.Lokator_C|GetCone (Variables|Default|GetSelectedLokator)) false false))
            (:Is%20Not%20Valid
              _))
          (bind _output_get (Variables|Default|SetSelectedLokator _lokator))
          (Rendering|SetVisibility (Variables|/Game/Blueprints/Lokator/Lokator.Lokator_C|GetCone _output_get) true false))))))

(event Input|KeyboardEvents|SpaceBar
  (params (Key :type Key%20Structure :default "AnyKey"))
  (bind _returnvalue (Game|GetPlayerController 0))
  (bind _array (Utilities|Array|MakeArray "ObjectTypeQuery7"))
  (bind (_hitresult _returnvalue_2) (Class|PlayerController|GetHitResultUnderCursorforObjects _returnvalue _array false))
  (bind _impactpoint (Collision|BreakHitResult _hitresult))
  ;[1 1 1] Spawn Lokator
  (:Pressed
    (if _returnvalue_2
      (bind _returnvalue_3 (Game|SpawnActorfromClass "/Game/Blueprints/Lokator/Lokator.Lokator_C" (Math|Transform|MakeTransform _impactpoint (Math|Rotator|MakeRotfromZX (Math|Vector|Normalize _impactpoint) (Math|Random|RandomUnitVector))) "AlwaysSpawn" 0 0))
      (Variables|/Game/Blueprints/Lokator/Lokator.Lokator_C|SetLokators _returnvalue_3 self)
      (Utilities|Array|Add (Variables|Default|GetLokators) _returnvalue_3))))

(fn ConstructionScript)

(fn FindClosestLokator
  (params (Position :type Vector))
  (for _array_element (Variables|Default|GetLokators)
    (if (Utilities|IsValid (LocalVariables|GetClosestLokator))
      (if (< (LocalVariables|GetClosestDistance) (Math|Vector|DotProduct (Math|Vector|Normalize (Transformation|GetActorLocation _array_element)) (Math|Vector|Normalize Position)))
        (LocalVariables|SetClosestLokator _array_element)
        (LocalVariables|SetClosestDistance (Math|Vector|DotProduct (Math|Vector|Normalize (Transformation|GetActorLocation _array_element)) (Math|Vector|Normalize Position))))
      (else
        (LocalVariables|SetClosestLokator _array_element)
        (LocalVariables|SetClosestDistance (Math|Vector|DotProduct (Math|Vector|Normalize (Transformation|GetActorLocation _array_element)) (Math|Vector|Normalize Position))))))
  (return (LocalVariables|GetClosestLokator)))